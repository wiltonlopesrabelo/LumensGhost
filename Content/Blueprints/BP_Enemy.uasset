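; BP_Enemy is a ghost enemy that chases the player and ends the game on contact.
; On BeginPlay it repeatedly uses AI MoveTo toward a random navigable point near the player's current location, restarting on both success and failure.
; Overlapping the player character disables the player controller's move input and displays the UI_GameOver widget, without destroying the character.
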(event `self.ReceiveBeginPlay`
  (bind _returnvalue (`GameplayStatics.GetPlayerCharacter` 0))
  ; Movimento do Ghost
  (`/Engine/EditorBlueprintResources/StandardMacros.IsValid` _returnvalue
    (:`Is Valid`
      (bind _randomlocation (`NavigationSystemV1.K2_GetRandomLocationInNavigableRadius` (`self.K2_GetActorLocation` _returnvalue) 50.0 null null :!label _label))
      (`|AIMoveTo` self _randomlocation null
        (:`OnSuccess`
          (goto _label))
        (:`OnFail`
          (goto _label))))))

(event `self.ReceiveActorBeginOverlap`
  (params (OtherActor :type "Actor Object Reference"))
  ; Ghost ao tocar personagem destroe o mesmo
  (if (== OtherActor (`GameplayStatics.GetPlayerCharacter` 0))
    (`Controller.SetIgnoreMoveInput` (`GameplayStatics.GetPlayerController` 0) true)
    (bind _returnvalue (`|CreateWidget` "/Game/UI/UI_GameOver.UI_GameOver_C"))
    (`UserWidget.AddToPlayerScreen` _returnvalue 0)))

(fn `UserConstructionScript`)