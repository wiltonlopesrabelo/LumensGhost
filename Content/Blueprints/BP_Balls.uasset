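; BP_Balls is a collectible ball that the player picks up by touching it, driving the win condition.
; A Sphere hit from the player character increments the Balls counter on BP_FirstPersonCharacter and destroys the ball.
; When the counter reaches three, it shows the UI_Victory widget, disables the player's move input and destroys every BP_Enemy actor.
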(event `self.Sphere.OnComponentHit`
  (params (HitComponent :type "PrimitiveComponent Object Reference") (OtherActor :type "Actor Object Reference") (OtherComp :type "PrimitiveComponent Object Reference") (NormalImpulse :type "Vector Structure") (Hit :type "HitResult Structure (by ref)"))
  ;[0.001686 0.15 0.09971 0.5] Quando o jogador encosta na bola
  (if (== OtherActor (`GameplayStatics.GetPlayerCharacter` 0))
    (bind _asbp_first_person_character (cast `/Game/FirstPerson/Blueprints/BP_FirstPersonCharacter` (`GameplayStatics.GetPlayerCharacter` 0)))
    (bind _result (`/Engine/EditorBlueprintResources/StandardMacros.IncrementInt` (`/Game/FirstPerson/Blueprints/BP_FirstPersonCharacter.Balls` _asbp_first_person_character))
      (:`  `
        (`self.K2_DestroyActor`)
        ;[0 0.05153 0.15 0.5] Quando todas as bolas são recuperadas
        (if (== _result 3)
          (bind _returnvalue (`|CreateWidget` "/Game/UI/UI_Victory.UI_Victory_C"))
          (`UserWidget.AddToPlayerScreen` _returnvalue 0)
          (`Controller.SetIgnoreMoveInput` (`GameplayStatics.GetPlayerController` 0) true)
          (bind _outactors (`GameplayStatics.GetAllActorsOfClass` "/Game/Blueprints/BP_Enemy.BP_Enemy_C"))
          (`self.K2_DestroyActor` _outactors))))))

(fn `UserConstructionScript`)